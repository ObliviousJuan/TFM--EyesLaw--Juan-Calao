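; Interactable button actor that opens the matching door when the player presses it.
; On Interact it searches all Door actors for the first whose DoorValue equals its ButtonValue, calls OpenDoor and blends the player's view to that door.
; A box trigger shows and hides a P_Interact prompt widget, created at BeginPlay, while the player character overlaps it.
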(event OnComponentBeginOverlap(Box)
  (params (OverlappedComponent :type Primitive%20Component%20Object%20Reference) (OtherActor :type Actor%20Object%20Reference) (OtherComp :type Primitive%20Component%20Object%20Reference) (OtherBodyIndex :type Integer) (bFromSweep :type Boolean) (SweepResult :type Hit%20Result%20Structure%20%28by%20ref%29))
  (if (== OtherActor (Game|GetPlayerCharacter 0))
    (UserInterface|Viewport|AddtoViewport (Variables|Default|GetP_Interact) 0)))

(event OnComponentEndOverlap(Box)
  (params (OverlappedComponent :type Primitive%20Component%20Object%20Reference) (OtherActor :type Actor%20Object%20Reference) (OtherComp :type Primitive%20Component%20Object%20Reference) (OtherBodyIndex :type Integer))
  (if (== (Game|GetPlayerCharacter 0) OtherActor)
    (Widget|RemovefromParent (Variables|Default|GetP_Interact))))

(event EventBeginPlay
  (bind _returnvalue (UserInterface|CreateWidget "/Game/Blueprint/InteraccionPuertas/P_Interact.P_Interact_C"))
  (Variables|Default|SetP_Interact _returnvalue))

(event EventInteract
  (params (Player :type Character%20Object%20Reference))
  ;[1 1 1] Oprimir
  (bind _outactors (Actor|GetAllActorsOfClass "/Game/Blueprint/InteraccionPuertas/Door.Door_C"))
  (bind _array_element (Utilities|Array|ForEachLoopwithBreak _outactors :!label _label)
    (:LoopBody
      (if (== (Variables|/Game/Blueprint/InteraccionPuertas/Door.Door_C|GetDoor%20Value _array_element) (Variables|Default|GetButtonValue))
        (Default|OpenDoor _array_element Player)
        (Game|Player|SetViewTargetwithBlend (Game|GetPlayerController 0) _array_element 0.0 "VTBlend_Linear" 0.0 false)
        (goto _label Break)))))

(fn ConstructionScript)