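; Player character with flipbook sprite that moves on the world X/Y axes, fires chargeable projectiles and interacts with objects.
; Tick switches Run/Idle flipbooks by velocity and snaps control yaw to face horizontal movement.
; Left click spawns a bullet, starts its charge and re-pins it to the Projectile component through a recursive Delay while charging.
; E messages the first overlapping InteractInterface actor; Lookat rotates the character toward a target.
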(event Custom|Animacion
  ;[1 1 1] Animacion
  (Sprite|SetFlipbook (Variables|Default|GetSprite) (select (> (Math|Vector|VectorLength (Variables|/Script/Engine.MovementComponent|GetVelocity (Variables|Character|GetCharacterMovement))) 0.0) "/Game/Sprites/Run.Run" "/Game/Sprites/Idle.Idle")))

(event Custom|Rotacion
  ;[1 1 1] Rotacion de personaje
  (Utilities|IsValid (Pawn|GetController)
    (:Is%20Valid
      (Math|Float|CompareFloat (.X (Math|Vector|BreakVector (Variables|/Script/Engine.MovementComponent|GetVelocity (Variables|Character|GetCharacterMovement)))) 0.0
        (:>
          (Pawn|SetControlRotation (Pawn|GetController) (Math|Rotator|MakeRotator 0.0 0.0 0.0)))
        (:<
          (Pawn|SetControlRotation (Pawn|GetController) (Math|Rotator|MakeRotator 0.0 0.0 1.8e+02)))))))

(event Custom|UpdateBulletLocation
  (bind _bullet (Variables|Default|GetBullet))
  (Transformation|SetActorLocation _bullet (Transformation|GetWorldLocation (Variables|Default|GetProjectile)) false false)
  (if (Variables|/Game/Blueprint/Projectile.Projectile_C|GetCharging _bullet)
    (Utilities|FlowControl|Delay 0.1)
    (CallFunction|UpdateBulletLocation)))

(event EventBeginPlay)

(event Collision|EventActorBeginOverlap
  (params (OtherActor :type Actor%20Object%20Reference)))

(event EventTick
  (params (DeltaSeconds :type Float%20%28single-precision%29))
  ;[1 1 1] Animacion
  (CallFunction|Animacion)
  (CallFunction|Rotacion))

(event EventLookat
  (params (Target :type Vector :default "0, 0, 0"))
  (bind _returnvalue (Transformation|GetActorLocation))
  (Transformation|SetActorRotation (Math|Rotator|FindLookatRotation (Math|Vector|MakeVector (.x _returnvalue) (.y _returnvalue) 0.0) (Math|Vector|MakeVector (.x Target) (.y Target) 0.0))))

(event Input|AxisEvents|InputAxisDerecha
  (params (AxisValue :type Float%20%28single-precision%29))
  ;[1 1 1] Movimiento
  (Pawn|Input|AddMovementInput "1.000000,0.000000,0.000000" AxisValue false))

(event Input|AxisEvents|InputAxisArriba
  (params (AxisValue :type Float%20%28single-precision%29))
  ;[1 1 1] Movimiento
  (Pawn|Input|AddMovementInput "0.000000,-1.000000,0.000000" AxisValue false))

(event Input|KeyboardEvents|E
  (params (Key :type Key%20Structure :default "None"))
  ;[1 1 1] Interaccion
  (:Pressed
    (bind _array_element (Utilities|Array|ForEachLoopwithBreak (Collision|GetOverlappingActors 0 :!class /Script/Engine.Actor) :!label _label)
      (:LoopBody
        (if (Utilities|DoesObjectImplementInterface _array_element "/Game/Blueprint/InteraccionPuertas/InteractInterface.InteractInterface_C")
          (Class|InteractInterface|Interact(Message) _array_element self)
          (goto _label Break))))))

(event Input|MouseEvents|LeftMouseButton
  (params (Key :type Key%20Structure :default "None"))
  (bind _projectile (Variables|Default|GetProjectile))
  (bind _returnvalue (Transformation|GetWorldTransform _projectile))
  (:Pressed
    (bind _returnvalue_2 (Game|SpawnActorfromClass "/Game/Blueprint/Projectile.Projectile_C" (Math|Transform|MakeTransform (.location _returnvalue) (.rotation _returnvalue) "0.500000,0.500000,0.500000") "AlwaysSpawn" "MultiplyWithRoot" 0 0))
    (bind _output_get (Variables|Default|SetBullet _returnvalue_2))
    (Class|BulletBehaviour|Charge(Message) _output_get)
    (CallFunction|UpdateBulletLocation)))

(fn ConstructionScript)